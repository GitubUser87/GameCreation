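; BP_NPC_Child1 is a child NPC blueprint for Scenario 5 that runs a click-through dialogue with the player.
; Each Talk event plays a click sound, advances TalkIndex and shows that Dialogue2 entry in a lazily created Dialogue_Wid while ignoring move input.
; Once the lines run out, it removes the widget, restores movement, destroys itself and sets TalkedToo on BP_ThirdPersonCharacter.
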(event `/Game/Scenarios/Scenario_4_Content/BP_Dialogue.Talk`
  (bind _returnvalue (`GameplayStatics.GetPlayerController` 0))
  ;[1 1 1] This will get the text box to display the text left in the dialogue array.
  (`GameplayStatics.PlaySound2D` "/Engine/VREditor/Sounds/VR_click1.VR_click1" 1.0 1.0 0.0 null null)
  (`/Engine/EditorBlueprintResources/StandardMacros.IncrementInt` (`self.TalkIndex`)
    (:`  `
      (if (< (`self.TalkIndex`) (`KismetArrayLibrary.Array_Length` (`self.Dialogue2`)))
        (`self.UI`
          (:`then`
            _)
          (:`else`
            (bind _returnvalue_2 (`|CreateWidget` "/Game/Scenarios/Scenario_4_Content/Dialogue_Wid.Dialogue_Wid_C" (`GameplayStatics.GetPlayerController` 0)))
            (bind _output_get (set `self.UI` _returnvalue_2))
            (`UserWidget.AddToViewport` _output_get 0)))
        (`TextBlock.SetText` (`/Game/Scenarios/Scenario_4_Content/Dialogue_Wid.TalkText` (`self.UI`)) (`KismetTextLibrary.Conv_StringToText` (`|GetArrayItem` (`self.Dialogue2`) (`self.TalkIndex`))))
        (`Controller.SetIgnoreMoveInput` _returnvalue true)
        (else
          (`Widget.RemoveFromParent` (`self.UI`))
          (`Controller.ResetIgnoreMoveInput` _returnvalue)
          (`self.K2_DestroyActor`)
          (bind _asbp_third_person_character (cast `/Game/ThirdPerson/Blueprints/BP_ThirdPersonCharacter` (`GameplayStatics.GetPlayerCharacter` 0)))
          (set `/Game/ThirdPerson/Blueprints/BP_ThirdPersonCharacter.Talked too?` true _asbp_third_person_character))))))

(fn `UserConstructionScript`
  (`parent.UserConstructionScript`))