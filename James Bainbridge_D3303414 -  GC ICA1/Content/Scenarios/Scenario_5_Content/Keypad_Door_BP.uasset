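; A keypad-locked door Blueprint that opens for the third-person character only once its Correct flag is set.
; On box overlap, an unlocked door slides its cube downward via a timeline with a sound, while a locked one shows the keypad widget with cursor and UI-only input.
; Leaving the box reverses the timeline and, after retriggerable delays, resets the DoOnce gates guarding the sound and widget.
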(event `self.Box.OnComponentBeginOverlap`
  (params (OverlappedComponent :type "PrimitiveComponent Object Reference") (OtherActor :type "Actor Object Reference") (OtherComp :type "PrimitiveComponent Object Reference") (OtherBodyIndex :type Integer) (bFromSweep :type Boolean) (SweepResult :type "HitResult Structure (by ref)"))
  (bind _returnvalue (`GameplayStatics.GetPlayerController` 0))
  ;[1 1 1] This will check to see if the code has been correctly inputted if not it will open the widget, if it has then it will open the door. Also added in reverse function.
  (cast `/Game/ThirdPerson/Blueprints/BP_ThirdPersonCharacter` OtherActor)
  (if (`self.Correct?`)
    (bind (_direction _open_track) (`Timeline|Open_Door` :!label _label)
      (:`Update`
        (`SceneComponent.K2_SetRelativeLocation` (`self.Cube`) (`KismetMathLibrary.VLerp` (0.0 0.0 0.0) (0.0 0.0 -400.0) _open_track) false false)
        (`/Engine/EditorBlueprintResources/StandardMacros.DoOnce` false :!label _label_2
          (:`Completed`
            (`GameplayStatics.PlaySound2D` "/Engine/VREditor/Sounds/UI/Dockable_Window_Open.Dockable_Window_Open" 1.0 1.0 0.0 null null)))))
    (else
      (`/Engine/EditorBlueprintResources/StandardMacros.DoOnce` false :!label _label_3
        (:`Completed`
          (bind _returnvalue_2 (`|CreateWidget` "/Game/Scenarios/Scenario_5_Content/Keypad_Wid.Keypad_Wid_C" (`GameplayStatics.GetPlayerController` 0)))
          (`UserWidget.AddToViewport` _returnvalue_2 0)
          (set `PlayerController.bShowMouseCursor` true _returnvalue)
          (`WidgetBlueprintLibrary.SetInputMode_UIOnlyEx` _returnvalue _returnvalue_2))))))

(event `self.Box.OnComponentEndOverlap`
  (params (OverlappedComponent :type "PrimitiveComponent Object Reference") (OtherActor :type "Actor Object Reference") (OtherComp :type "PrimitiveComponent Object Reference") (OtherBodyIndex :type Integer))
  ;[1 1 1] This will check to see if the code has been correctly inputted if not it will open the widget, if it has then it will open the door. Also added in reverse function.
  (`|ExecutionSequence`
    (:`then_0`
      (`KismetSystemLibrary.RetriggerableDelay` 0.7)
      (goto _label_3 :!via `Reset`))
    (:`then_1`
      (goto _label :!via `Reverse`))
    (:`then_2`
      (`KismetSystemLibrary.RetriggerableDelay` 1.0)
      (goto _label_2 :!via `Reset`))))

(fn `UserConstructionScript`)