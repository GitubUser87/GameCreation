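; Collectable pickup actor for Scenario 5 that spins in place until the player collects it.
; When a BP_ThirdPersonCharacter overlaps its Box, it increments that character's Pickups and decrements PickupsLeft, plays a pickup sound and destroys itself.
; Tick applies a local yaw rotation scaled by the Rotation variable and delta time, keeping the spin frame-rate independent.
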(event `self.Box.OnComponentBeginOverlap`
  (params (OverlappedComponent :type "PrimitiveComponent Object Reference") (OtherActor :type "Actor Object Reference") (OtherComp :type "PrimitiveComponent Object Reference") (OtherBodyIndex :type Integer) (bFromSweep :type Boolean) (SweepResult :type "HitResult Structure (by ref)"))
  ;[1 1 1] This will add collectables to the players total.
  (bind _asbp_third_person_character (cast `/Game/ThirdPerson/Blueprints/BP_ThirdPersonCharacter` OtherActor))
  (set `/Game/ThirdPerson/Blueprints/BP_ThirdPersonCharacter.Pickups` (+ (`/Game/ThirdPerson/Blueprints/BP_ThirdPersonCharacter.Pickups` _asbp_third_person_character) 1) _asbp_third_person_character)
  (set `/Game/ThirdPerson/Blueprints/BP_ThirdPersonCharacter.PickupsLeft` (- (`/Game/ThirdPerson/Blueprints/BP_ThirdPersonCharacter.PickupsLeft` _asbp_third_person_character) 1) _asbp_third_person_character)
  (`GameplayStatics.PlaySound2D` "/Engine/VREditor/Sounds/UI/Dockable_Window_Pick_Up.Dockable_Window_Pick_Up" 1.0 1.0 0.0 null null)
  (`self.K2_DestroyActor`))

(event `self.ReceiveTick`
  (params (DeltaSeconds :type "Float (single-precision)"))
  ;[1 1 1] This will cause the pickup to spin.
  (`self.K2_AddActorLocalRotation` (`KismetMathLibrary.MakeRotator` 0.0 0.0 (* (`self.Rotation`) DeltaSeconds))))

(fn `UserConstructionScript`)