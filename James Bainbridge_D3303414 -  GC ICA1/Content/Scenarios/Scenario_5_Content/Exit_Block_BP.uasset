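; Exit_Block_BP is an exit blocker that lets the player leave only after collecting five pickups.
; When the player character overlaps its Box with five pickups, a success sound plays and, once only, a message prints and the Unlock timeline lowers the Cube.
; Otherwise a DoOnce gates a failure sound and a printout of pickups left, re-armed by a retriggerable one-second delay after the player exits the Box.
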(event `self.Box.OnComponentBeginOverlap`
  (params (OverlappedComponent :type "PrimitiveComponent Object Reference") (OtherActor :type "Actor Object Reference") (OtherComp :type "PrimitiveComponent Object Reference") (OtherBodyIndex :type Integer) (bFromSweep :type Boolean) (SweepResult :type "HitResult Structure (by ref)"))
  ;[1 1 1] This will allow the player to leave once they have found the collectables but will prevent them from leaving if they do not.
  (bind _asbp_third_person_character (cast `/Game/ThirdPerson/Blueprints/BP_ThirdPersonCharacter` OtherActor))
  (if (== (`/Game/ThirdPerson/Blueprints/BP_ThirdPersonCharacter.Pickups` _asbp_third_person_character) 5)
    (`GameplayStatics.PlaySound2D` "/Engine/EditorSounds/Notifications/CompileSuccess.CompileSuccess" 1.0 1.0 0.0 null null)
    (`/Engine/EditorBlueprintResources/StandardMacros.DoOnce` false
      (:`Completed`
        (`KismetSystemLibrary.PrintString` "Well done.")
        (bind (_direction _open_track) (`Timeline|Unlock`)
          (:`Update`
            (`SceneComponent.K2_SetRelativeLocation` (`self.Cube`) (`KismetMathLibrary.VLerp` (0.0 0.0 0.0) (0.0 0.0 -340.0) _open_track) false false)))))
    (else
      (`/Engine/EditorBlueprintResources/StandardMacros.DoOnce` false :!label _label
        (:`Completed`
          (bind _asbp_third_person_character_2 (cast `/Game/ThirdPerson/Blueprints/BP_ThirdPersonCharacter` (`GameplayStatics.GetPlayerCharacter` 0)))
          (`GameplayStatics.PlaySound2D` "/Engine/EditorSounds/Notifications/CompileFailed.CompileFailed" 1.0 1.0 0.0 null null)
          (`KismetSystemLibrary.PrintString` (`KismetStringLibrary.Conv_IntToString` (`/Game/ThirdPerson/Blueprints/BP_ThirdPersonCharacter.PickupsLeft` _asbp_third_person_character_2))))))))

(event `self.Box.OnComponentEndOverlap`
  (params (OverlappedComponent :type "PrimitiveComponent Object Reference") (OtherActor :type "Actor Object Reference") (OtherComp :type "PrimitiveComponent Object Reference") (OtherBodyIndex :type Integer))
  ;[1 1 1] This will allow the player to leave once they have found the collectables but will prevent them from leaving if they do not.
  (cast `/Game/ThirdPerson/Blueprints/BP_ThirdPersonCharacter` OtherActor)
  (`KismetSystemLibrary.RetriggerableDelay` 1.0)
  (goto _label :!via `Reset`))

(fn `UserConstructionScript`)