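; Key pickup Blueprint for Scenario 3 that grants the player a key.
; It creates an E_wid prompt on BeginPlay and shows or hides it as player 0 enters or leaves its Box trigger.
; Interact casts to BP_ThirdPersonCharacter, sets HasKey, plays a 2D sound and destroys the actor.
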(event `/Game/Scenarios/Scenario_3_Content/Interact.Interact`
  (params (Player :type "Character Object Reference"))
  ;[1 1 1] This will give the player the key upon the player picking it up.
  (bind _asbp_third_person_character (cast `/Game/ThirdPerson/Blueprints/BP_ThirdPersonCharacter` Player))
  (set `/Game/ThirdPerson/Blueprints/BP_ThirdPersonCharacter.HasKey?` true _asbp_third_person_character)
  (`GameplayStatics.PlaySound2D` "/Engine/VREditor/Sounds/UI/Dockable_Window_Open.Dockable_Window_Open" 1.0 1.0 0.0 null null)
  (`self.K2_DestroyActor`))

(event `self.ReceiveBeginPlay`
  (bind _returnvalue (`|CreateWidget` "/Game/ThirdPerson/Blueprints/E_wid.E_wid_C"))
  (set `self.InteractPrompt` _returnvalue))

(event `self.Box.OnComponentBeginOverlap`
  (params (OverlappedComponent :type "PrimitiveComponent Object Reference") (OtherActor :type "Actor Object Reference") (OtherComp :type "PrimitiveComponent Object Reference") (OtherBodyIndex :type Integer) (bFromSweep :type Boolean) (SweepResult :type "HitResult Structure (by ref)"))
  (if (== OtherActor (`GameplayStatics.GetPlayerCharacter` 0))
    (`UserWidget.AddToViewport` (`self.InteractPrompt`) 0)))

(event `self.Box.OnComponentEndOverlap`
  (params (OverlappedComponent :type "PrimitiveComponent Object Reference") (OtherActor :type "Actor Object Reference") (OtherComp :type "PrimitiveComponent Object Reference") (OtherBodyIndex :type Integer))
  (if (== (`GameplayStatics.GetPlayerCharacter` 0) OtherActor)
    (`Widget.RemoveFromParent` (`self.InteractPrompt`))))

(fn `UserConstructionScript`)