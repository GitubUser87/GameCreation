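; Interactable button Blueprint that opens the door whose DoorValue matches its ButtonValue.
; The trigger box shows and hides an interact prompt widget as the player enters and leaves.
; Interact animates the button with a timeline that reverses after a delay, then searches all Door_BP actors.
; On the first match it plays a click, calls OpenDoor and disables the box's collision.
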(event `/Game/Scenarios/Scenario_3_Content/Interact.Interact`
  (params (Player :type "Character Object Reference"))
  ;[1 1 1] This will allow the button to be pressed which will then open the door.
  (`|ExecutionSequence`
    (:`then_0`
      (bind (_direction _pressed_track) (`Timeline|Pressed` :!label _label)
        (:`Update`
          (`SceneComponent.K2_SetRelativeLocation` (`self.Button1`) (`KismetMathLibrary.MakeVector` 0.0 (`KismetMathLibrary.Lerp` 0.0 -10.0 _pressed_track)) false false)
          (`KismetSystemLibrary.Delay` 2.0)
          (goto _label :!via `Reverse`))))
    (:`then_1`
      (bind _outactors (`GameplayStatics.GetAllActorsOfClass` "/Game/Scenarios/Scenario_3_Content/Door_BP.Door_BP_C"))
      (for _array_element _outactors
        (if (== (`/Game/Scenarios/Scenario_3_Content/Door_BP.Door value` _array_element) (`self.Button value`))
          (`GameplayStatics.PlaySound2D` "/Engine/VREditor/Sounds/UI/Click_on_Button.Click_on_Button" 1.0 1.0 0.0 null null)
          (`/Game/Scenarios/Scenario_3_Content/Door_BP.Open door` _array_element)
          (`PrimitiveComponent.SetCollisionEnabled` (`self.Box`) "NoCollision")
          (break))))))

(event `self.ReceiveBeginPlay`
  ;[1 1 1] Create interact widget
  (bind _returnvalue (`|CreateWidget` "/Game/ThirdPerson/Blueprints/E_wid.E_wid_C"))
  (set `self.InteractPrompt` _returnvalue))

(event `self.Box.OnComponentBeginOverlap`
  (params (OverlappedComponent :type "PrimitiveComponent Object Reference") (OtherActor :type "Actor Object Reference") (OtherComp :type "PrimitiveComponent Object Reference") (OtherBodyIndex :type Integer) (bFromSweep :type Boolean) (SweepResult :type "HitResult Structure (by ref)"))
  ;[1 1 1] Create interact widget
  (if (== OtherActor (`GameplayStatics.GetPlayerCharacter` 0))
    (`UserWidget.AddToViewport` (`self.InteractPrompt`) 0)))

(event `self.Box.OnComponentEndOverlap`
  (params (OverlappedComponent :type "PrimitiveComponent Object Reference") (OtherActor :type "Actor Object Reference") (OtherComp :type "PrimitiveComponent Object Reference") (OtherBodyIndex :type Integer))
  ;[1 1 1] Create interact widget
  (if (== (`GameplayStatics.GetPlayerCharacter` 0) OtherActor)
    (`Widget.RemoveFromParent` (`self.InteractPrompt`))))

(fn `UserConstructionScript`)