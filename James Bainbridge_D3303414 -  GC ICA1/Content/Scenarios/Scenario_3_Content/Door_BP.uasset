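; Scenario 3 door Blueprint that slides open downward when its Opendoor event is called.
; A timeline lerps the Cube's relative location along Z and clears the Opening flag.
; While Opening is true, the player character entering the Box triggers a sound and an on-screen prompt to press the button.
; A DoOnce limits repeat prompts and resets after a short retriggerable delay when the player leaves.
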(event `Open door`
  ;[1 1 1] This will open the door when the event has been called for.
  (bind (_direction _open_track) (`Timeline|Open_door`)
    (:`Update`
      (`SceneComponent.K2_SetRelativeLocation` (`self.Cube`) (`KismetMathLibrary.VLerp` (0.0 0.0 0.0) (0.0 0.0 -340.0) _open_track) false false)
      (set `self.Opening?` false))))

(event `self.Box.OnComponentBeginOverlap`
  (params (OverlappedComponent :type "PrimitiveComponent Object Reference") (OtherActor :type "Actor Object Reference") (OtherComp :type "PrimitiveComponent Object Reference") (OtherBodyIndex :type Integer) (bFromSweep :type Boolean) (SweepResult :type "HitResult Structure (by ref)"))
  ;[1 1 1] This will tell the player to press the button to open the door.
  (cast `/Game/ThirdPerson/Blueprints/BP_ThirdPersonCharacter` OtherActor)
  (if (`self.Opening?`)
    (`/Engine/EditorBlueprintResources/StandardMacros.DoOnce` false :!label _label
      (:`Completed`
        (`GameplayStatics.PlaySound2D` "/Engine/EditorSounds/Notifications/CompileFailed.CompileFailed" 1.0 1.0 0.0 null null)
        (`KismetSystemLibrary.PrintString` "Press button to open door.")))))

(event `self.Box.OnComponentEndOverlap`
  (params (OverlappedComponent :type "PrimitiveComponent Object Reference") (OtherActor :type "Actor Object Reference") (OtherComp :type "PrimitiveComponent Object Reference") (OtherBodyIndex :type Integer))
  ;[1 1 1] This will tell the player to press the button to open the door.
  (cast `/Game/ThirdPerson/Blueprints/BP_ThirdPersonCharacter` OtherActor)
  (`KismetSystemLibrary.RetriggerableDelay` 0.5)
  (goto _label :!via `Reset`))

(fn `UserConstructionScript`)