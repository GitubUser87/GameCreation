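; Pressure plate actor that sinks under the third-person character and opens matching pressure doors in the level.
; Overlapping Trigger plays a timeline that lowers the plate mesh, with a DoOnce-gated click sound, and leaving reverses it.
; A separate Trigger_Door overlap searches all Pressure_Door_BP actors and opens those whose PressureDoorValue equals this plate's PressureValue.
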(event `self.Trigger.OnComponentBeginOverlap`
  (params (OverlappedComponent :type "PrimitiveComponent Object Reference") (OtherActor :type "Actor Object Reference") (OtherComp :type "PrimitiveComponent Object Reference") (OtherBodyIndex :type Integer) (bFromSweep :type Boolean) (SweepResult :type "HitResult Structure (by ref)"))
  ;[1 1 1] This will trigger the pressure plate animation when the player steps on the trigger box.
  (cast `/Game/ThirdPerson/Blueprints/BP_ThirdPersonCharacter` OtherActor)
  (bind (_direction _pressure_track) (`Timeline|Pressure` :!label _label)
    (:`Update`
      (`SceneComponent.K2_SetRelativeLocation` (`self.Plate`) (`KismetMathLibrary.MakeVector` 0.0 0.0 (`KismetMathLibrary.Lerp` 17.0 -3.0 _pressure_track)) false false)
      (`/Engine/EditorBlueprintResources/StandardMacros.DoOnce` false
        (:`Completed`
          (`GameplayStatics.PlaySound2D` "/Engine/VREditor/Sounds/UI/Click_on_Button.Click_on_Button" 1.0 1.0 0.0 null null))))))

(event `self.Trigger.OnComponentEndOverlap`
  (params (OverlappedComponent :type "PrimitiveComponent Object Reference") (OtherActor :type "Actor Object Reference") (OtherComp :type "PrimitiveComponent Object Reference") (OtherBodyIndex :type Integer))
  ;[1 1 1] This will trigger the pressure plate animation when the player steps on the trigger box.
  (cast `/Game/ThirdPerson/Blueprints/BP_ThirdPersonCharacter` OtherActor)
  (goto _label :!via `Reverse`))

(event `self.Trigger_Door.OnComponentBeginOverlap`
  (params (OverlappedComponent :type "PrimitiveComponent Object Reference") (OtherActor :type "Actor Object Reference") (OtherComp :type "PrimitiveComponent Object Reference") (OtherBodyIndex :type Integer) (bFromSweep :type Boolean) (SweepResult :type "HitResult Structure (by ref)"))
  ;[1 1 1] This will call to the pressure door and allow it to be open.
  (cast `/Game/ThirdPerson/Blueprints/BP_ThirdPersonCharacter` OtherActor)
  (bind _outactors (`GameplayStatics.GetAllActorsOfClass` "/Game/Scenarios/Scenario_3_Content/Pressure_Door_BP.Pressure_Door_BP_C"))
  (for _array_element _outactors
    (if (== (`/Game/Scenarios/Scenario_3_Content/Pressure_Door_BP.Pressure door value` _array_element) (`self.Pressure_Value`))
      (`/Game/Scenarios/Scenario_3_Content/Pressure_Door_BP.Open Pressure door` _array_element))))

(fn `UserConstructionScript`)