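; Keycard door Blueprint that slides open when a player carrying the key enters its trigger box.
; Box overlap checks the character's HasKey; if set, a one-time gate plays a sound and a timeline lerps the cube downward.
; Without the key, a second DoOnce plays a failure sound and prints a hint to find the keycard.
; Leaving the box resets that hint gate after a short retriggerable delay, preventing rapid repeats.
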(event `self.Box.OnComponentEndOverlap`
  (params (OverlappedComponent :type "PrimitiveComponent Object Reference") (OtherActor :type "Actor Object Reference") (OtherComp :type "PrimitiveComponent Object Reference") (OtherBodyIndex :type Integer))
  ;[1 1 1] This will open the door if the player has the key or tell them to go find the key if not.
  (cast `/Game/ThirdPerson/Blueprints/BP_ThirdPersonCharacter` OtherActor)
  (`KismetSystemLibrary.RetriggerableDelay` 0.5)
  (goto _label :!via `Reset`))

(event `self.Box.OnComponentBeginOverlap`
  (params (OverlappedComponent :type "PrimitiveComponent Object Reference") (OtherActor :type "Actor Object Reference") (OtherComp :type "PrimitiveComponent Object Reference") (OtherBodyIndex :type Integer) (bFromSweep :type Boolean) (SweepResult :type "HitResult Structure (by ref)"))
  ;[1 1 1] This will open the door if the player has the key or tell them to go find the key if not.
  (bind _asbp_third_person_character (cast `/Game/ThirdPerson/Blueprints/BP_ThirdPersonCharacter` OtherActor))
  (if (`/Game/ThirdPerson/Blueprints/BP_ThirdPersonCharacter.HasKey?` _asbp_third_person_character)
    (`/Engine/EditorBlueprintResources/StandardMacros.DoOnce` false
      (:`Completed`
        (`GameplayStatics.PlaySound2D` "/Engine/VREditor/Sounds/UI/Dockable_Window_Drop.Dockable_Window_Drop" 1.0 1.0 0.0 null null)
        (bind (_direction _key_door_track) (`Timeline|Key Door`)
          (:`Update`
            (`SceneComponent.K2_SetRelativeLocation` (`self.Cube`) (`KismetMathLibrary.VLerp` (0.0 0.0 0.0) (0.0 0.0 -340.0) _key_door_track) false false)))))
    (else
      (`/Engine/EditorBlueprintResources/StandardMacros.DoOnce` false :!label _label
        (:`Completed`
          (`GameplayStatics.PlaySound2D` "/Engine/EditorSounds/Notifications/CompileFailed.CompileFailed" 1.0 1.0 0.0 null null)
          (`KismetSystemLibrary.PrintString` "Go find the keycard"))))))

(fn `UserConstructionScript`)