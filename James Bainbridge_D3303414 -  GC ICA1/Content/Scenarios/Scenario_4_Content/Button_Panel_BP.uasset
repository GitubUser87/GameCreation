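; Interactable button panel that opens linked Button_Door_BP doors once its power count reaches three.
; Its box overlap shows or hides an interact prompt widget for the player character.
; Each Interact increments and prints a click count, raises Power and plays a click sound.
; It then searches all doors for a matching button value and, at exactly three Power, opens them, disables box collision and plays a success sound.
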(event `/Game/Scenarios/Scenario_4_Content/Interact_BP.Interact`
  (params (Player :type "Character Object Reference"))
  ;[1 1 1] Interact
  (bind _result (`/Engine/EditorBlueprintResources/StandardMacros.IncrementInt` (`self.Clicked`))
    (:`  `
      (bind _output_get (set `self.Clicked` _result))
      (`KismetSystemLibrary.PrintString` (`KismetStringLibrary.Conv_IntToString` _output_get))
      (bind _result_2 (`/Engine/EditorBlueprintResources/StandardMacros.IncrementFloat` (`self.Power`))
        (:`  `
          (set `self.Power` _result_2)
          (`GameplayStatics.PlaySound2D` "/Engine/VREditor/Sounds/UI/Click_on_Button.Click_on_Button" 1.0 1.0 0.0 null null)
          (bind _outactors (`GameplayStatics.GetAllActorsOfClass` "/Game/Scenarios/Scenario_4_Content/Button_Door_BP.Button_Door_BP_C"))
          (for _array_element _outactors
            (if (and (== (`/Game/Scenarios/Scenario_4_Content/Button_Door_BP.Button_Door_Value` _array_element) (`self.Button_Value`)) (== (`self.Power`) 3.0))
              (`/Game/Scenarios/Scenario_4_Content/Button_Door_BP.Open Button Door` _array_element)
              (`PrimitiveComponent.SetCollisionEnabled` (`self.Box`) "NoCollision")
              (`GameplayStatics.PlaySound2D` "/Engine/EditorSounds/Notifications/CompileSuccess.CompileSuccess" 1.0 1.0 0.0 null null))))))))

(event `self.ReceiveBeginPlay`
  ;[1 1 1] Creates an interact widget
  (bind _returnvalue (`|CreateWidget` "/Game/ThirdPerson/Blueprints/E_wid.E_wid_C"))
  (set `self.InteractPrompt` _returnvalue))

(event `self.Box.OnComponentBeginOverlap`
  (params (OverlappedComponent :type "PrimitiveComponent Object Reference") (OtherActor :type "Actor Object Reference") (OtherComp :type "PrimitiveComponent Object Reference") (OtherBodyIndex :type Integer) (bFromSweep :type Boolean) (SweepResult :type "HitResult Structure (by ref)"))
  ;[1 1 1] Creates an interact widget
  (if (== OtherActor (`GameplayStatics.GetPlayerCharacter` 0))
    (`UserWidget.AddToViewport` (`self.InteractPrompt`) 0)))

(event `self.Box.OnComponentEndOverlap`
  (params (OverlappedComponent :type "PrimitiveComponent Object Reference") (OtherActor :type "Actor Object Reference") (OtherComp :type "PrimitiveComponent Object Reference") (OtherBodyIndex :type Integer))
  ;[1 1 1] Creates an interact widget
  (if (== (`GameplayStatics.GetPlayerCharacter` 0) OtherActor)
    (`Widget.RemoveFromParent` (`self.InteractPrompt`))))

(fn `UserConstructionScript`)