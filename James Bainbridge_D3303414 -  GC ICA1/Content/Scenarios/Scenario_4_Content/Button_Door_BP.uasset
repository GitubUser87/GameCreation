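; Scenario 4 door Blueprint that stays shut until its OpenButtonDoor event is called, telling the player a device must be hacked.
; OpenButtonDoor plays a timeline that lerps the door downward and disables the Box trigger's collision.
; While the trigger is active, player overlap plays an error sound and prints the hint through a DoOnce, reset by a retriggerable delay after exit to limit repeats.
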(event `Open Button Door`
  ;[1 1 1] Open door
  (bind (_direction _opentrack) (`Timeline|Open_Door` :!via `PlayFromStart`)
    (:`Update`
      (`SceneComponent.K2_SetRelativeLocation` (`self.Door`) (`KismetMathLibrary.VLerp` (0.0 0.0 0.0) (0.0 0.0 -300.0) _opentrack) false false)
      (`PrimitiveComponent.SetCollisionEnabled` (`self.Box`) "NoCollision"))))

(event `self.Box.OnComponentBeginOverlap`
  (params (OverlappedComponent :type "PrimitiveComponent Object Reference") (OtherActor :type "Actor Object Reference") (OtherComp :type "PrimitiveComponent Object Reference") (OtherBodyIndex :type Integer) (bFromSweep :type Boolean) (SweepResult :type "HitResult Structure (by ref)"))
  ;[1 1 1] Open door
  (cast `/Game/ThirdPerson/Blueprints/BP_ThirdPersonCharacter` OtherActor)
  (`/Engine/EditorBlueprintResources/StandardMacros.DoOnce` false :!label _label
    (:`Completed`
      (`GameplayStatics.PlaySound2D` "/Engine/EditorSounds/Notifications/CompileFailed.CompileFailed" 1.0 1.0 0.0 null null)
      (`KismetSystemLibrary.PrintString` "You must hack a device to open this door."))))

(event `self.Box.OnComponentEndOverlap`
  (params (OverlappedComponent :type "PrimitiveComponent Object Reference") (OtherActor :type "Actor Object Reference") (OtherComp :type "PrimitiveComponent Object Reference") (OtherBodyIndex :type Integer))
  ;[1 1 1] Open door
  (cast `/Game/ThirdPerson/Blueprints/BP_ThirdPersonCharacter` OtherActor)
  (`KismetSystemLibrary.RetriggerableDelay` 0.5)
  (goto _label :!via `Reset`))

(fn `UserConstructionScript`)