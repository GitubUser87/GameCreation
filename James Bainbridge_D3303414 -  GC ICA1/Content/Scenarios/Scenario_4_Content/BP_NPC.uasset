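; BP_NPC is a scenario NPC that shows a bobbing monitor and an interact prompt while the player overlaps its trigger.
; Each Talk call plays a click and advances through the Dialogue array in an on-screen text widget, ignoring move input and setting the character's Talking flag.
; After the last line it removes the widget, restores input and destroys itself.
; A Moving timeline drives the bob, toggling direction after a delay.
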(event `/Game/Scenarios/Scenario_4_Content/BP_Dialogue.Talk`
  (bind _returnvalue (`GameplayStatics.GetPlayerController` 0))
  ;[1 1 1] This will get the text box to display the text left in the dialogue array.
  (`GameplayStatics.PlaySound2D` "/Engine/VREditor/Sounds/VR_click1.VR_click1" 1.0 1.0 0.0 null null)
  (`/Engine/EditorBlueprintResources/StandardMacros.IncrementInt` (`self.TalkIndex`)
    (:`  `
      (if (< (`self.TalkIndex`) (`KismetArrayLibrary.Array_Length` (`self.Dialogue`)))
        (`self.UI`
          (:`then`
            _)
          (:`else`
            (bind _returnvalue_2 (`|CreateWidget` "/Game/Scenarios/Scenario_4_Content/Dialogue_Wid.Dialogue_Wid_C" (`GameplayStatics.GetPlayerController` 0)))
            (bind _output_get (set `self.UI` _returnvalue_2))
            (`UserWidget.AddToViewport` _output_get 0)))
        (`TextBlock.SetText` (`/Game/Scenarios/Scenario_4_Content/Dialogue_Wid.TalkText` (`self.UI`)) (`KismetTextLibrary.Conv_StringToText` (`|GetArrayItem` (`self.Dialogue`) (`self.TalkIndex`))))
        (`Controller.SetIgnoreMoveInput` _returnvalue true)
        (bind _asbp_third_person_character (cast `/Game/ThirdPerson/Blueprints/BP_ThirdPersonCharacter` (`GameplayStatics.GetPlayerCharacter` 0)))
        (set `/Game/ThirdPerson/Blueprints/BP_ThirdPersonCharacter.Talking?` true _asbp_third_person_character)
        (else
          (`Widget.RemoveFromParent` (`self.UI`))
          (`Controller.ResetIgnoreMoveInput` _returnvalue)
          (bind _asbp_third_person_character_2 (cast `/Game/ThirdPerson/Blueprints/BP_ThirdPersonCharacter` (`GameplayStatics.GetPlayerCharacter` 0)))
          (set `/Game/ThirdPerson/Blueprints/BP_ThirdPersonCharacter.Talking?` false _asbp_third_person_character_2)
          (`self.K2_DestroyActor`))))))

(event `self.ReceiveBeginPlay`
  ;[1 1 1] Interact
  (bind _returnvalue (`|CreateWidget` "/Game/ThirdPerson/Blueprints/E_wid.E_wid_C"))
  (set `self.Prompt` _returnvalue)
  ;[1 1 1] This allows the monitor to bob up and down.
  (bind (_direction _moving) (`Timeline|Moving` :!label _label)
    (:`Update`
      (`SceneComponent.K2_SetRelativeLocation` (`self.Test`) _moving false false)
      (`KismetSystemLibrary.Delay` 0.5)
      (if (`self.IsLooped`)
        (set `self.IsLooped` false)
        (goto _label :!via `Reverse`)
        (else
          (set `self.IsLooped` true)
          (goto _label))))))

(event `self.E Trigger.OnComponentBeginOverlap`
  (params (OverlappedComponent :type "PrimitiveComponent Object Reference") (OtherActor :type "Actor Object Reference") (OtherComp :type "PrimitiveComponent Object Reference") (OtherBodyIndex :type Integer) (bFromSweep :type Boolean) (SweepResult :type "HitResult Structure (by ref)"))
  ;[1 1 1] Interact
  (if (== OtherActor (`GameplayStatics.GetPlayerCharacter` 0))
    (`UserWidget.AddToViewport` (`self.Prompt`) 0)))

(event `self.E Trigger.OnComponentEndOverlap`
  (params (OverlappedComponent :type "PrimitiveComponent Object Reference") (OtherActor :type "Actor Object Reference") (OtherComp :type "PrimitiveComponent Object Reference") (OtherBodyIndex :type Integer))
  ;[1 1 1] Interact
  (if (== (`GameplayStatics.GetPlayerCharacter` 0) OtherActor)
    (`Widget.RemoveFromParent` (`self.Prompt`))))

(fn `UserConstructionScript`)